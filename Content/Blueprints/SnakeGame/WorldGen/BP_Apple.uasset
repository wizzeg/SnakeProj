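; BP_Apple is the Blueprint for the apple pickup in the snake game, adding an explosion effect.
; It caches the SnakeGameStateBase at BeginPlay to read the apples-to-eat and apples-eaten counts.
; PlayParticleEffect spawns the explosion emitter slightly above the apple only when the target exceeds the eaten count plus one, so the final required apple gets no effect.
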(event `self.ReceiveBeginPlay`
  (bind _assnake_game_state_base (cast `SnakeGameStateBase` (`GameplayStatics.GetGameState`))))

(event `self.PlayParticleEffect`
  (bind _returnvalue (`SnakeGameStateBase.GetApplesToEat` (stale `self.ReceiveBeginPlay` _assnake_game_state_base)))
  (bind _returnvalue_2 (`SnakeGameStateBase.GetApplesEaten` (stale `self.ReceiveBeginPlay` _assnake_game_state_base)))
  (if (> _returnvalue (+ _returnvalue_2 1))
    (`GameplayStatics.SpawnEmitterAtLocation` "/Game/StarterContent/Particles/P_Explosion.P_Explosion" (+ (`self.K2_GetActorLocation`) (0.0 0.0 25.0)))))

(fn `UserConstructionScript`)