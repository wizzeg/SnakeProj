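; Player controller for the snake game that takes keyboard input for two players through a single controller.
; On BeginPlay it sets game-only input, adds the IMC_SnakeKB Enhanced Input mapping context and caches the first player pawn as BP_PawnManager, printing setup status.
; Each player's four directional input actions call MovePlayer1 or MovePlayer2 with the matching direction.
; Leftover ActionValue branches and a SetUpInput call are unconnected and never run.
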(event `self.ReceiveBeginPlay`
  (bind _returnvalue (pcsubsystem `EnhancedInputLocalPlayerSubsystem` self))
  (`WidgetBlueprintLibrary.SetInputMode_GameOnly` self)
  (`/Engine/EditorBlueprintResources/StandardMacros.IsValid` _returnvalue
    (:`Is Valid`
      (`EnhancedInputSubsystemInterface.AddMappingContext` _returnvalue "/Game/Blueprints/SnakeGame/MoveSystem/IMC_SnakeKB.IMC_SnakeKB" 0 (struct))
      (bind _asbp_pawn_manager (cast `/Game/Blueprints/SnakeGame/Pawns/BP_PawnManager` (`GameplayStatics.GetPlayerPawn` 0))
        (:`then`
          (set `self.PawnManager` _asbp_pawn_manager)
          (`KismetSystemLibrary.PrintString` "Successfully added KeyboardContext"))
        (:`CastFailed`
          (`KismetSystemLibrary.PrintString` "Failed cast to PawnManager (BP Error)"))))
    (:`Is Not Valid`
      (`KismetSystemLibrary.PrintText` "Failed Input setup" true true (struct :`R` 1.0 :`B` 0.235015 :`A` 1.0)))))

(event `self.ReceiveTick`
  (params (DeltaSeconds :type "Float (single-precision)")))

(event `EnhancedInput|/Game/Blueprints/SnakeGame/MoveSystem/IA_Player1Up`
  (params (ActionValue :type Boolean) (ElapsedSeconds :type "Float (double-precision)") (TriggeredSeconds :type "Float (double-precision)") (InputAction :type "InputAction Object Reference" :default "/Game/Blueprints/SnakeGame/MoveSystem/IA_Player1Up.IA_Player1Up"))
  (:`Triggered`
    (`self.MovePlayer1` "UP")))

(event `EnhancedInput|/Game/Blueprints/SnakeGame/MoveSystem/IA_Player1Down`
  (params (ActionValue :type Boolean) (ElapsedSeconds :type "Float (double-precision)") (TriggeredSeconds :type "Float (double-precision)") (InputAction :type "InputAction Object Reference" :default "/Game/Blueprints/SnakeGame/MoveSystem/IA_Player1Down.IA_Player1Down"))
  (:`Triggered`
    (`self.MovePlayer1` "DOWN")))

(event `EnhancedInput|/Game/Blueprints/SnakeGame/MoveSystem/IA_Player1Left`
  (params (ActionValue :type Boolean) (ElapsedSeconds :type "Float (double-precision)") (TriggeredSeconds :type "Float (double-precision)") (InputAction :type "InputAction Object Reference" :default "/Game/Blueprints/SnakeGame/MoveSystem/IA_Player1Left.IA_Player1Left"))
  (:`Triggered`
    (`self.MovePlayer1` "LEFT")))

(event `EnhancedInput|/Game/Blueprints/SnakeGame/MoveSystem/IA_Player1Right`
  (params (ActionValue :type Boolean) (ElapsedSeconds :type "Float (double-precision)") (TriggeredSeconds :type "Float (double-precision)") (InputAction :type "InputAction Object Reference" :default "/Game/Blueprints/SnakeGame/MoveSystem/IA_Player1Right.IA_Player1Right"))
  (:`Triggered`
    (`self.MovePlayer1` "RIGHT")))

(event `EnhancedInput|/Game/Blueprints/SnakeGame/MoveSystem/IA_Player2Up`
  (params (ActionValue :type Boolean) (ElapsedSeconds :type "Float (double-precision)") (TriggeredSeconds :type "Float (double-precision)") (InputAction :type "InputAction Object Reference" :default "/Game/Blueprints/SnakeGame/MoveSystem/IA_Player2Up.IA_Player2Up"))
  (:`Triggered`
    (`self.MovePlayer2` "UP")))

(event `EnhancedInput|/Game/Blueprints/SnakeGame/MoveSystem/IA_Player2Down`
  (params (ActionValue :type Boolean) (ElapsedSeconds :type "Float (double-precision)") (TriggeredSeconds :type "Float (double-precision)") (InputAction :type "InputAction Object Reference" :default "/Game/Blueprints/SnakeGame/MoveSystem/IA_Player2Down.IA_Player2Down"))
  (:`Triggered`
    (`self.MovePlayer2` "DOWN")))

(event `EnhancedInput|/Game/Blueprints/SnakeGame/MoveSystem/IA_Player2Left`
  (params (ActionValue :type Boolean) (ElapsedSeconds :type "Float (double-precision)") (TriggeredSeconds :type "Float (double-precision)") (InputAction :type "InputAction Object Reference" :default "/Game/Blueprints/SnakeGame/MoveSystem/IA_Player2Left.IA_Player2Left"))
  (:`Triggered`
    (`self.MovePlayer2` "LEFT")))

(event `EnhancedInput|/Game/Blueprints/SnakeGame/MoveSystem/IA_Player2Right`
  (params (ActionValue :type Boolean) (ElapsedSeconds :type "Float (double-precision)") (TriggeredSeconds :type "Float (double-precision)") (InputAction :type "InputAction Object Reference" :default "/Game/Blueprints/SnakeGame/MoveSystem/IA_Player2Right.IA_Player2Right"))
  (:`Triggered`
    (`self.MovePlayer2` "RIGHT")))

(fn `UserConstructionScript`)