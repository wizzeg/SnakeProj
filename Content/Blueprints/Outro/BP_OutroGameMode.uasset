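; Game mode for the snake game's outro screen, showing final scores and handling the return to the main menu.
; On BeginPlay it creates the outro widget, switches to UI-only input with a visible cursor, and fills in scores from the game instance: a combined total in co-op, separate player scores in versus.
; It listens to the state machine subsystem, resetting the game and opening the main menu level on entering the Mainmenu state.
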(event `self.ReceiveBeginPlay`
  (bind _returnvalue (`GameplayStatics.GetPlayerController` 0))
  (bind _returnvalue_2 (`|CreateWidget` "/Game/Blueprints/Outro/BP_Outro.BP_Outro_C"))
  (`UserWidget.AddToViewport` _returnvalue_2 10)
  (`WidgetBlueprintLibrary.SetInputMode_UIOnlyEx` _returnvalue _returnvalue_2)
  (set `PlayerController.bShowMouseCursor` true _returnvalue)
  (add `StateMachineSubsystem.OnStateChanged` (subsystem `StateMachineSubsystem`) (`|CreateDelegate` :!event `OnStateChanged`))
  (bind _assnake_game_instance (cast `SnakeGameInstance` (`GameplayStatics.GetGameInstance`)))
  (bind _returnvalue_3 (`SnakeGameInstance.GetScores` _assnake_game_instance))
  (if (`SnakeGameInstance.bIsCoop` _assnake_game_instance)
    (`/Game/Blueprints/Outro/BP_Outro.SetIntro` _returnvalue_2 "Coop Score")
    (`/Game/Blueprints/Outro/BP_Outro.SetPlayer2Text` _returnvalue_2 "")
    (bind _output (`|GetArrayItem` _returnvalue_3))
    (bind _output_2 (`|GetArrayItem` _returnvalue_3 1))
    (`/Game/Blueprints/Outro/BP_Outro.SetPlayer1Text` _returnvalue_2 (`KismetStringLibrary.Concat_StrStr` "Coop Score: " (`KismetStringLibrary.Conv_IntToString` (+ _output _output_2))))
    (else
      (`/Game/Blueprints/Outro/BP_Outro.SetIntro` _returnvalue_2 "Versus Score")
      (`/Game/Blueprints/Outro/BP_Outro.SetPlayer1Text` _returnvalue_2 (`KismetStringLibrary.Concat_StrStr` "Player1 Score: " (`KismetStringLibrary.Conv_IntToString` _output)))
      (`/Game/Blueprints/Outro/BP_Outro.SetPlayer2Text` _returnvalue_2 (`KismetStringLibrary.Concat_StrStr` "Player2 Score: " (`KismetStringLibrary.Conv_IntToString` _output_2))))))

(event `OnStateChanged`
  (params (ExitState :type "EStates Enum" :default "mainmenu") (EnterState :type "EStates Enum" :default "mainmenu"))
  (`|ExecutionSequence`
    (:`then_0`
      (switch `EStates` ExitState))
    (:`then_1`
      (switch `EStates` EnterState
        (:`mainmenu`
          (`SnakeGameInstance.ResetGame` (stale `self.ReceiveBeginPlay` _assnake_game_instance))
          (`GameplayStatics.OpenLevelBySoftObjectPtr` "/Game/MainMenu.MainMenu"))))))

(fn `UserConstructionScript`)