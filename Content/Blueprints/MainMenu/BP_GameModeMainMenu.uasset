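; Main menu game mode for a snake game that shows the menu widget and launches the match.
; On BeginPlay it creates the menu container and binds to the state machine subsystem's state changes.
; Entering Playing reads both players from the menu held by the game state, passes them to the game instance as snake controllers, then opens the snake level.
; Failed casts only print an error.
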(event `self.ReceiveBeginPlay`
  (bind _returnvalue (`|CreateWidget` "/Game/Blueprints/MainMenu/Widgets/BP_MainMenuContainer.BP_MainMenuContainer_C"))
  (`UserWidget.AddToViewport` _returnvalue 0)
  (add `StateMachineSubsystem.OnStateChanged` (subsystem `StateMachineSubsystem`) (`|CreateDelegate` :!event `OnStateChanged`)))

(event `OnStateChanged`
  (params (ExitState :type "EStates Enum" :default "mainmenu") (EnterState :type "EStates Enum" :default "mainmenu"))
  (`|ExecutionSequence`
    (:`then_0`
      (switch `EStates` ExitState))
    (:`then_1`
      (switch `EStates` EnterState
        (:`playing`
          (bind _asmain_menu_game_state_base (cast `MainMenuGameStateBase` (`GameplayStatics.GetGameState`))
            (:`then`
              (bind _returnvalue (`MainMenuGameStateBase.GetMainMenu` _asmain_menu_game_state_base))
              (bind _asbp_main_menu_container (cast `/Game/Blueprints/MainMenu/Widgets/BP_MainMenuContainer` _returnvalue)
                (:`then`
                  (bind (_player1 _player2) (`/Game/Blueprints/MainMenu/Widgets/BP_MainMenuContainer.GetPlayers` _asbp_main_menu_container))
                  (bind _assnake_game_instance (cast `SnakeGameInstance` (`GameplayStatics.GetGameInstance`))
                    (:`then`
                      (`SnakeGameInstance.AddSnakeControllers` _assnake_game_instance (`|MakeArray` _player1 _player2))
                      (`GameplayStatics.OpenLevelBySoftObjectPtr` "/Game/SnakeLevel.SnakeLevel"))
                    (:`CastFailed`
                      (`KismetSystemLibrary.PrintString` "FAILD TO CAST GAME INSTANCE"))))
                (:`CastFailed`
                  (`KismetSystemLibrary.PrintString` "FAILED CASTING MAINMENU CONTAINER"))))
            (:`CastFailed`
              (`KismetSystemLibrary.PrintString` "FAILED CASTING GAMESTATE"))))))))

(fn `UserConstructionScript`)